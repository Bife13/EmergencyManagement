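; Hospital hover-info Blueprint that shows a tooltip widget when the cursor is over its collision, with an optional icon.
; On BeginPlay it passes itself, the tooltip text and the tinted icon image to the widgets via message calls, or hides the icon.
; Collision cursor events and the MouseWidgetInteraction callback share OnCollision and OnWidget flags to keep the tooltip visible while the mouse moves onto a widget.
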(event `self.ReceiveBeginPlay`
  (bind _returnvalue (`WidgetComponent.GetUserWidgetObject` (`self.Icon`)))
  (bind _returnvalue_2 (`WidgetComponent.GetUserWidgetObject` (`self.Tooltip`)))
  ;[1 1 1] set tooltip text
  (message `/Game/Balduin/BPI_tooltip.tooltipReference` _returnvalue_2 self)
  (message `/Game/Balduin/BPI_tooltip.tooltipTextReference` _returnvalue_2 (`self.Tooltip Text`))
  (if (`self.icon `)
    ;[1 1 1] set icon image
    (message `/Game/Balduin/BPI_tooltip.tooltipReference` _returnvalue self)
    (message `/Game/Balduin/BPI_tooltip.iconImageReference` _returnvalue (`self.Icon Image`) (`self.In Brush Tint Specified Color`))
    (else
      (`SceneComponent.SetVisibility` (`self.Icon`) false false))))

(event `self.Collision.OnBeginCursorOver`
  (params (TouchedComponent :type "PrimitiveComponent Object Reference"))
  ;[1 1 1] Visibility if mouse over collision / widgets
  (`SceneComponent.SetVisibility` (`self.Tooltip`) true false)
  (set `self.on collision` true))

(event `self.Collision.OnEndCursorOver`
  (params (TouchedComponent :type "PrimitiveComponent Object Reference"))
  ;[1 1 1] Visibility if mouse over collision / widgets
  (if (not (`self.on widget`))
    (set `self.on collision` false)
    (`SceneComponent.SetVisibility` (`self.Tooltip`) false false :!label _label)))

(event `/Game/Balduin/BPI_tooltip.mouseWidgetInteraction`
  (params (`mouse over widget` :type Boolean))
  ;[1 1 1] Visibility if mouse over collision / widgets
  (bind _output_get (set `self.on widget` `mouse over widget`))
  (if (not (and _output_get (`self.on collision`)))
    (goto _label)))

(fn `UserConstructionScript`)
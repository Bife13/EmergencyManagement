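; TestRoom is a clickable room actor that links the hospital UI to the node editor.
; On BeginPlay, after a short delay, it looks up and caches the HospitalUI and NodeEditorV1 widgets.
; Cursor hover sends the actor's object name to the hospital UI as text.
; Clicking its Cube with the button whose display name matches ClickButton makes the node editor create an action widget.
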(event `self.ReceiveBeginPlay`
  (`KismetSystemLibrary.Delay` 0.1)
  (bind _foundwidgets (`WidgetBlueprintLibrary.GetAllWidgetsOfClass` "/Game/NodeEditor/Widgets/HospitalUI.HospitalUI_C" false))
  (set `self.HospitalUI` (`|GetArrayItem` _foundwidgets))
  (bind _foundwidgets_2 (`WidgetBlueprintLibrary.GetAllWidgetsOfClass` "/Game/NodeEditor/Old/NodeEditorV1.NodeEditorV1_C" false))
  (set `self.NodeEditor` (`|GetArrayItem` _foundwidgets_2)))

(event `self.ReceiveActorBeginCursorOver`
  (bind _hospitalui (`self.HospitalUI`))
  (if (`KismetSystemLibrary.IsValid` _hospitalui)
    (`/Game/NodeEditor/Widgets/HospitalUI.ChangeText` _hospitalui (`KismetTextLibrary.Conv_StringToText` (`KismetSystemLibrary.GetObjectName` self)))))

(event `self.Cube.OnClicked`
  (params (TouchedComponent :type "PrimitiveComponent Object Reference") (ButtonPressed :type "Key Structure"))
  (if (`KismetTextLibrary.EqualEqual_TextText` (`KismetInputLibrary.Key_GetDisplayName` ButtonPressed false) (`self.ClickButton`))
    (`/Game/NodeEditor/Old/NodeEditorV1.CreateActionWidgetFromHospital` (`self.NodeEditor`))))

(fn `UserConstructionScript`)
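; Player Blueprint that toggles the node editor UI and controls camera zoom.
; On BeginPlay it caches the first NodeEditorV2 widget found, and the B key switches that widget between visible and hidden.
; While the editor is not visible, mouse wheel input scaled by ZoomSpeed changes the CameraArm length, which is clamped so it never drops below zero.
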(event `self.ReceiveBeginPlay`
  (bind _foundwidgets (`WidgetBlueprintLibrary.GetAllWidgetsOfClass` "/Game/Mona/NodeEditorV2.NodeEditorV2_C" false))
  (set `self.NodeEditor` (`|GetArrayItem` _foundwidgets)))

(event `Key|B` :paused true
  (params (Key :type "Key Structure"))
  (bind _nodeeditor (`self.NodeEditor`))
  (:`Pressed`
    (if (`Widget.IsVisible` _nodeeditor)
      (`Widget.SetVisibility` _nodeeditor "Hidden")
      (else
        (`Widget.SetVisibility` _nodeeditor "Visible")))))

(event `InputAxisKey|MouseWheelAxis`
  (params (AxisValue :type "Float (single-precision)"))
  (bind _cameraarm (`self.CameraArm`))
  (bind _returnvalue (+ (`SpringArmComponent.TargetArmLength` _cameraarm) (* AxisValue (`self.ZoomSpeed`))))
  (if (`Widget.IsVisible` (`self.NodeEditor`))
    _
    (elif (>= _returnvalue 0.0)
      (set `SpringArmComponent.TargetArmLength` _returnvalue _cameraarm)
      (else
        (set `SpringArmComponent.TargetArmLength` 0.0 _cameraarm)))))

(event `Key|SpaceBar`
  (params (Key :type "Key Structure")))

(fn `UserConstructionScript`)